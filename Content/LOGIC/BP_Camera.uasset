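; BP_Camera drives the level's CameraActor, turning it every tick to face the player pawn.
; CE_MoveCamera slides the camera to a target X/Y at its current height, lerping along the CameraSlide timeline.
; When the slide finishes, it spawns a BP_Levy at the target at a fixed height and stores it as CurLevy.
; Logic to scale and rotate that levy is disconnected and never runs.
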(event `self.ReceiveBeginPlay`
  (bind _returnvalue (`GameplayStatics.GetActorOfClass` "/Script/Engine.CameraActor"))
  (set `self.Camera` _returnvalue))

(event `self.ReceiveTick`
  (params (DeltaSeconds :type "Float (single-precision)"))
  (bind _camera (`self.Camera`))
  (`self.K2_SetActorRotation` _camera (`KismetMathLibrary.Conv_VectorToRotator` (- (`self.K2_GetActorLocation` (`GameplayStatics.GetPlayerPawn` 0)) (`self.K2_GetActorLocation` _camera))) false))

(event `CE_MoveCamera`
  (params (TargetLocation :type "Vector Structure"))
  (bind _camera (`self.Camera`))
  (bind _targetlocation (`self.TargetLocation`))
  (bind (_returnvalue_x _returnvalue_y _returnvalue_z) (`KismetMathLibrary.BreakVector` (`self.K2_GetActorLocation` _camera)))
  (set `self.TargetLocation` (`KismetMathLibrary.MakeVector` (.x TargetLocation) (.y TargetLocation) _returnvalue_z))
  (set `self.StartLocation` (`self.K2_GetActorLocation` _camera))
  (bind (_direction _linear) (`Timeline|CameraSlide` :!via `PlayFromStart`)
    (:`Update`
      (`self.K2_SetActorLocation` _camera (`KismetMathLibrary.VLerp` (`self.StartLocation`) _targetlocation _linear) false false))
    (:`Finished`
      (bind _returnvalue (`|SpawnActorFromClass` "/Game/LOGIC/BP_Levy.BP_Levy_C" (`KismetMathLibrary.MakeTransform` (`KismetMathLibrary.MakeVector` (.x _targetlocation) (.y _targetlocation) 45.0)) "Undefined" "OverrideRootScale" null null))
      (set `self.CurLevy` _returnvalue))))

(fn `UserConstructionScript`)