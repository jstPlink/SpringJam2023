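; Sprout actor that switches between a stump and a large birch tree in one of three color kinds, with random yaw and scale.
; SelectKind inherits the parent's kind with a generation-dependent probability, otherwise picks another, then applies the stump look.
; While ControlLevy is on, Tick stretches a spawned BP_Levy toward the player, feeding normalized distance to its material.
; Switching it off aims the levy at the new sprout and thickens it.
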(event `Grow`
  (bind _sm_treebirch_04 (`self.SM_TreeBirch_04`))
  (`KismetSystemLibrary.Delay` 0.2)
  (`StaticMeshComponent.SetStaticMesh` _sm_treebirch_04 "/Game/DreamscapeSeries/DreamscapeMeadows/Meshes/Trees/SM_Tree_Large_02.SM_Tree_Large_02")
  (`PrimitiveComponent.SetMaterial` _sm_treebirch_04 0 (select `int` (`self.Kind`) :`0` "/Game/DreamscapeSeries/DreamscapeMeadows/Materials/Trees/MI_TreeLeaf_Birch_Red.MI_TreeLeaf_Birch_Red" :`1` "/Game/DreamscapeSeries/DreamscapeMeadows/Materials/Trees/MI_TreeLeaf_Birch.MI_TreeLeaf_Birch" :`2` "/Game/DreamscapeSeries/DreamscapeMeadows/Materials/Trees/MI_TreeLeaf_Birch_Yellow.MI_TreeLeaf_Birch_Yellow" :!type "MaterialInterface Object Reference")))

(event `self.ReceiveBeginPlay`
  (bind _sm_treebirch_04 (`self.SM_TreeBirch_04`))
  (bind _returnvalue (* (`KismetMathLibrary.RandomFloatInRange` 0.8 1.2) 0.4))
  (`parent.ReceiveBeginPlay`)
  (`SceneComponent.K2_SetWorldRotation` _sm_treebirch_04 (`KismetMathLibrary.MakeRotator` 0.0 0.0 (`KismetMathLibrary.RandomFloatInRange` 0.0 180.0)) false false)
  (`SceneComponent.SetWorldScale3D` _sm_treebirch_04 (`KismetMathLibrary.MakeVector` _returnvalue _returnvalue _returnvalue)))

(event `Undo Grow`
  (bind _sm_treebirch_04 (`self.SM_TreeBirch_04`))
  (`StaticMeshComponent.SetStaticMesh` _sm_treebirch_04 "/Game/DreamscapeSeries/DreamscapeMeadows/Meshes/Props/SM_Tree_Stump_01.SM_Tree_Stump_01" :!label _label)
  (`PrimitiveComponent.SetMaterial` _sm_treebirch_04 0 (select `int` (`self.Kind`) :`0` "/Game/DreamscapeSeries/DreamscapeMeadows/Materials/Props/MI_Props_Tree_Stump_Brown.MI_Props_Tree_Stump_Brown" :`1` "/Game/DreamscapeSeries/DreamscapeMeadows/Materials/Props/MI_Props_Tree_Stump_White.MI_Props_Tree_Stump_White" :`2` "/Game/DreamscapeSeries/DreamscapeMeadows/Materials/Props/MI_Props_Tree_Stump_Yellow.MI_Props_Tree_Stump_Yellow" :!type "MaterialInterface Object Reference")))

(event `self.SelectKind`
  (params (ParentKind :type Integer))
  (set `self.Kind` (`KismetMathLibrary.SelectInt` ParentKind (mod (+ ParentKind (`KismetMathLibrary.RandomIntegerInRange` 1 2)) 3) (> (/ 0.5 (`KismetMathLibrary.MultiplyMultiply_FloatFloat` (`self.CurvaProbabilitàStessoTipo`) (`KismetMathLibrary.Conv_IntToDouble` (`self.Generazione`)))) (`KismetMathLibrary.RandomFloat`))))
  (goto _label))

(event `self.ReceiveTick`
  (params (DeltaSeconds :type "Float (single-precision)"))
  (bind _returnvalue (`self.K2_GetActorLocation`))
  (bind _returnvalue_2 (`GameplayStatics.GetPlayerPawn` 0))
  (bind _mylevy (`self.MyLevy`))
  (bind _returnvalue_3 (`self.K2_GetActorLocation` _returnvalue_2))
  (bind _returnvalue_4 (`KismetMathLibrary.Vector_Distance` _returnvalue_3 _returnvalue))
  (if (`self.ControlLevy`)
    ;[0.27 1 0.002064] levy rotation update
    (`/Engine/EditorBlueprintResources/StandardMacros.IsValid` _mylevy
      (:`Is Valid`
        (`MaterialInstanceDynamic.SetScalarParameterValue` (`/Game/LOGIC/BP_Levy.DynamicMaterialInstance` _mylevy) "Lenght" (/ _returnvalue_4 (`/Game/LOGIC/BP_ThirdPersonCharacter.DistanzaMax` (cast `/Game/LOGIC/BP_ThirdPersonCharacter` _returnvalue_2 :!pure true))))
        (bind _output_get (set `self.CurZScale` (/ _returnvalue_4 400.0)))
        (`SceneComponent.SetRelativeScale3D` (`/Game/LOGIC/BP_Levy.Cube` _mylevy) (`KismetMathLibrary.MakeVector` 1.0 1.0 _output_get))
        (`self.K2_SetActorRotation` _mylevy (`KismetMathLibrary.Conv_VectorToRotator` (- (- _returnvalue_3 (0.0 0.0 80.0)) _returnvalue)) false)))))

(event `CE_ControlLevy`
  (params (ControlLevy :type Boolean) (NewSprout :type "/Game/LOGIC/BP_Sprout Object Reference"))
  (bind _mylevy (`self.MyLevy`))
  (bind _output_get (set `self.ControlLevy` ControlLevy))
  (if _output_get
    (`/Engine/EditorBlueprintResources/StandardMacros.IsValid` _mylevy
      (:`Is Not Valid`
        ;[0.1968 0.249 1] spawn levy
        (bind _returnvalue (`|SpawnActorFromClass` "/Game/LOGIC/BP_Levy.BP_Levy_C" (`KismetMathLibrary.MakeTransform` (`KismetMathLibrary.MakeVector` (.x (`self.K2_GetActorLocation`)) (.y (`self.K2_GetActorLocation`)) (+ (.z (`self.K2_GetActorLocation`)) 40.0))) "Undefined" "OverrideRootScale" null null))
        (set `self.MyLevy` _returnvalue)))
    (else
      ;[0.148 1 0.07743] attach levy
      (`/Engine/EditorBlueprintResources/StandardMacros.IsValid` _mylevy
        (:`Is Valid`
          (`self.K2_SetActorRotation` _mylevy (`KismetMathLibrary.Conv_VectorToRotator` (- (`self.K2_GetActorLocation` NewSprout) (`self.K2_GetActorLocation`))) false)
          (`MaterialInstanceDynamic.SetScalarParameterValue` (`/Game/LOGIC/BP_Levy.DynamicMaterialInstance` _mylevy) "Lenght" 0.0)
          (`SceneComponent.SetRelativeScale3D` (`/Game/LOGIC/BP_Levy.Cube` (`self.MyLevy`)) (`KismetMathLibrary.MakeVector` 4.0 4.0 (`self.CurZScale`))))))))

(fn `UserConstructionScript`)