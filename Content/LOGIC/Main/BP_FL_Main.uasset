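; Blueprint function library with main shared helpers: a game mode getter and an array sort.
; FLGetGameMode returns the current game mode cast to BP_MainGameMode.
; SortArray is a hand-written bubble sort, ascending or descending, that swaps out-of-order neighbours and repeats passes until none swap or Tries runs out.
; It returns the new array with the remaining tries, so a low limit can leave it partly sorted.
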(fn `FL_GetGameMode`
  (returns (`AsBP Main Game Mode` :type "/Game/LOGIC/Main/BP_MainGameMode Object Reference"))
  (locals (GameModeRef :type "GameMode Object Reference"))
  (bind _asbp_main_game_mode (cast `/Game/LOGIC/Main/BP_MainGameMode` (`GameplayStatics.GetGameMode` null)))
  (return _asbp_main_game_mode))

(fn `SortArray`
  (params (Array :type "Array of Float (double-precision)") (Tries :type Integer) (Descending :type Boolean))
  (returns (NewArray :type "Array of Float (double-precision)") (RemainingTries :type Integer))
  (locals (Array1 :type "Array of Float (double-precision)") (CurIndex :type Integer) (CurValue :type "Float (double-precision)") (Array2 :type "Array of Float (double-precision)") (SwappedOnce :type Boolean) (Lastvalue :type "Float (double-precision)"))
  (bind _tries (`local.Tries`))
  (bind _lastvalue (`local.Lastvalue`))
  (bind _curvalue (`local.CurValue`))
  (bind _curvalue_2 (`local.CurValue`))
  (bind _array2 (`local.Array2`))
  (set `local.Array1` Array)
  (for (_array_element _array_index) (`local.Array1`) :!label _label
    (bind _output_get (set `local.CurIndex` _array_index))
    (set `local.CurValue` _array_element)
    (if (== _output_get 0)
      ;[1 1 1] ok il corrente è piu grande del precedente
      (`KismetArrayLibrary.Array_Add` (`local.Array2`) _curvalue_2 :!label _label_2)
      (set `local.Lastvalue` _curvalue_2)
      (elif (select `bool` (`local.Descending`) :`false` (>= _curvalue _lastvalue) :`true` (<= _curvalue _lastvalue))
        (goto _label_2)
        (else
          ;[1 1 1] setta il corrente valore al posto dell'index precedente
          (`KismetArrayLibrary.Array_Set` (`local.Array2`) (- (`local.CurIndex`) 1) (`local.CurValue`) true)
          ;[1 1 1] e setta il precedente al posto dell'attuale
          (`KismetArrayLibrary.Array_Set` (`local.Array2`) (`local.CurIndex`) (`local.Lastvalue`) true)
          (set `local.SwappedOnce` true)))))
  (if (`local.SwappedOnce`)
    (`/Engine/EditorBlueprintResources/StandardMacros.DecrementInt` _tries
      (:`  `
        (if (> Tries 0)
          (set `local.Array1` _array2)
          (`KismetArrayLibrary.Array_Clear` _array2)
          (set `local.SwappedOnce` false)
          (goto _label)
          (else
            _)))))
  (return _array2 _tries))