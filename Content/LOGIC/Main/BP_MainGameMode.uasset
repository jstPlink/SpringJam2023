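; Main game mode that drives a day-light cycle, a countdown timer and staged procedural growth of a bud-based structure.
; Tick steadily pitches the level's directional light, while a looping one-second timer decrements the countdown and only prints when time runs out.
; BeginPlay queues several generations, each calling GenerateChildren on pending leaf buds, yielding a tick every 25 buds and between generations to spread the load.
; CreateConnection is an empty stub.
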(event `self.ReceiveTick`
  (params (DeltaSeconds :type "Float (single-precision)"))
  (`self.K2_AddActorLocalRotation` (`self.DirectionalLight`) (`KismetMathLibrary.MakeRotator` 0.0 (* DeltaSeconds 0.6)) false false))

(event `self.ReceiveBeginPlay`
  (bind _returnvalue (`GameplayStatics.GetActorOfClass` "/Script/Engine.DirectionalLight"))
  (set `self.DirectionalLight` _returnvalue)
  (bind _returnvalue_2 (`KismetSystemLibrary.K2_SetTimerDelegate` (delegate `Countdown`) 1.0 true))
  (set `self.CountdownRef` _returnvalue_2)
  (`self.GenerateMultiple` (`self.InitialGenerations`)))

(event `Countdown`
  (bind _output_get (set `self.CountdownTime` (- (`self.CountdownTime`) 1)))
  (`KismetSystemLibrary.PrintString` (`KismetStringLibrary.Conv_IntToString` _output_get))
  (if (== _output_get 0)
    ;[1 1 1] Funzione Endgame
    (`KismetSystemLibrary.PrintString` "Time End" true true (struct :`R` 0.583 :`A` 1.0))))

(event `GenerateMultiple`
  (params (Generations :type Integer))
  (if (> Generations 0)
    (set `self.QueuedGenerations` (- Generations 1))
    (`self.GenerateOnce`)))

(event `CreateConnection`
  (params (NodeA :type "Actor Object Reference") (NodeB :type "Actor Object Reference")))

(event `GenerateOnce`
  (bind _queuedgenerations (`self.QueuedGenerations`))
  (bind _output_get (set `self.PendingBuds` (`self.LeafBuds`)))
  (set `self.LeafBuds` (`|MakeArray` null :!type "/Game/LOGIC/BP_Bud Object Reference"))
  (set `self.GenerationPage` 0)
  (bind _returnvalue (`KismetArrayLibrary.Array_Length` _output_get))
  (`KismetSystemLibrary.PrintString` (`KismetStringLibrary.Conv_IntToString` _returnvalue))
  (for _index (range (+ _returnvalue 1))
    (bind _output (`|GetArrayItem` (`self.PendingBuds`) _index))
    (if (`/Game/LOGIC/BP_Bud.PendingGeneration` _output)
      (`/Game/LOGIC/BP_Bud.GenerateChildren` _output)
      (bind _result (`/Engine/EditorBlueprintResources/StandardMacros.IncrementInt` (`self.GenerationPage`))
        (:`  `
          (if (== (mod _result 25) 0)
            (`KismetSystemLibrary.PrintString` "Hello")
            (`KismetSystemLibrary.DelayUntilNextTick`))))))
  (if (> _queuedgenerations 0)
    (`KismetSystemLibrary.DelayUntilNextTick`)
    (`/Engine/EditorBlueprintResources/StandardMacros.DecrementInt` _queuedgenerations
      (:`  `
        (`self.GenerateOnce`)))))

(fn `UserConstructionScript`)