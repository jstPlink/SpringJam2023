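; BP_PlayerCharacter is the player character, with axis-driven movement and look plus a Connect action for linking two world actors.
; Connect line-traces from the camera, and a FlipFlop stores hit actors tagged ConnectionNode alternately as Actor0 and Actor1.
; While both are valid, Tick traces between them each frame; the link appears only as a debug line, as the trace result is unused.
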(event `InputAxis|MoveUpDown`
  (params (AxisValue :type "Float (single-precision)"))
  (`self.AddMovementInput` (`self.GetActorForwardVector`) AxisValue))

(event `InputAxis|LookUpDown`
  (params (AxisValue :type "Float (single-precision)"))
  (`self.AddControllerPitchInput` AxisValue))

(event `self.ReceiveTick`
  (params (DeltaSeconds :type "Float (single-precision)"))
  (if (and (`KismetSystemLibrary.IsValid` (`self.Actor0`)) (`KismetSystemLibrary.IsValid` (`self.Actor1`)))
    (`KismetSystemLibrary.LineTraceSingle` :`Start` (`self.K2_GetActorLocation` (`self.Actor0`)) :`End` (`self.K2_GetActorLocation` (`self.Actor1`)) :`TraceChannel` "TraceTypeQuery1" :`DrawDebugType` "ForOneFrame")))

(event `InputAxis|MoveRightLeft`
  (params (AxisValue :type "Float (single-precision)"))
  (`self.AddMovementInput` (`self.GetActorRightVector`) AxisValue))

(event `InputAxis|LookRightLeft`
  (params (AxisValue :type "Float (single-precision)"))
  (`self.AddControllerYawInput` AxisValue))

(event `InputAction|Connect`
  (params (Key :type "Key Structure"))
  (bind _camera (`self.Camera`))
  (bind _returnvalue (`SceneComponent.K2_GetComponentLocation` _camera))
  (:`Pressed`
    (bind _outhit (`KismetSystemLibrary.LineTraceSingle` :`Start` _returnvalue :`End` (+ _returnvalue (* (`SceneComponent.GetForwardVector` _camera) (`self.RaycastDistance`))) :`TraceChannel` "TraceTypeQuery1" :`DrawDebugType` "ForDuration"))
    (if (`self.ActorHasTag` (`.HitActor` (`GameplayStatics.BreakHitResult` _outhit)) "ConnectionNode")
      (`/Engine/EditorBlueprintResources/StandardMacros.FlipFlop`
        (:`A`
          (set `self.Actor0` (`.HitActor` (`GameplayStatics.BreakHitResult` _outhit))))
        (:`B`
          (set `self.Actor1` (`.HitActor` (`GameplayStatics.BreakHitResult` _outhit))))))))

(fn `UserConstructionScript`)