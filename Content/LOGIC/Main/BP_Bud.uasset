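; BP_Bud is a self-replicating growth node that registers with BP_MainGameMode's PendingBuds on spawn.
; BeginPlay first runs a sphere trace and destroys the bud if a WorldDynamic object is within DistanzaMinima.
; GenerateChildren spawns a clamped random number of same-class buds in a yaw cone, aimed midway between outward-from-world-origin and the bud's forward vector.
; Each child repeats the spacing check, so growth spreads outward without crowding.
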(event `self.ReceiveBeginPlay`
  (`self.CheckOverlap` (`self.DistanzaMinima`))
  (`KismetArrayLibrary.Array_Add` (`/Game/LOGIC/Main/BP_MainGameMode.PendingBuds` (cast `/Game/LOGIC/Main/BP_MainGameMode` (`GameplayStatics.GetGameMode`) :!pure true)) self))

(event `GenerateChildren`
  (bind _angolocono (`self.AngoloCono`))
  (bind _figlimin (`self.FigliMin`))
  (bind _figlimax (`self.FigliMax`))
  (bind _returnvalue (`KismetMathLibrary.GreaterGreater_VectorRotator` (`KismetMathLibrary.VLerp` (`KismetMathLibrary.Vector_Normal2D` (`self.K2_GetActorLocation`)) (`self.GetActorForwardVector`) 0.5) (`KismetMathLibrary.MakeRotator` 0.0 0.0 (`KismetMathLibrary.RandomFloatInRange` (- 0.0 _angolocono) _angolocono))))
  (set `self.PendingGeneration` false)
  (for _ (range 1 (+ (`KismetMathLibrary.Clamp` (+ (`KismetMathLibrary.RandomIntegerInRange` _figlimin _figlimax) (`KismetMathLibrary.RandomIntegerInRange` _figlimin _figlimax)) (`self.FigliMin`) (`self.FigliMax`)) 1))
    (`|SpawnActorFromClass` (`GameplayStatics.GetObjectClass` self) (`KismetMathLibrary.MakeTransform` (+ (`self.K2_GetActorLocation`) (* _returnvalue (`KismetMathLibrary.RandomFloatInRange` (`self.DistanzaMinima`) (`self.LunghezzaInternaCono`)))) (`KismetMathLibrary.Conv_VectorToRotator` _returnvalue)) "Undefined" "OverrideRootScale" null null)))

(fn `CheckOverlap`
  (params (Radius :type "Float (single-precision)"))
  (bind _returnvalue (`self.K2_GetActorLocation`))
  (bind (_outhit _returnvalue_2) (`KismetSystemLibrary.SphereTraceSingleForObjects` _returnvalue _returnvalue Radius (`|MakeArray` "ObjectTypeQuery2" :!type "EObjectTypeQuery Enum")))
  (if _returnvalue_2
    (if false
      (`PrimitiveComponent.SetMaterial` (`self.Sphere`) 0 "/Engine/VREditor/BasicMeshes/MI_Cube_03.MI_Cube_03")
      (else
        (`self.K2_DestroyActor`))))
  (return))

(fn `UserConstructionScript`)