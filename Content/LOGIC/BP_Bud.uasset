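; BP_Bud is a node in procedural branching growth that registers itself in the game mode's LeafBuds and can spawn child buds.
; On BeginPlay a sphere trace destroys it when it overlaps nearby dynamic objects.
; GenerateChildren spawns random children in a cone biased away from world origin, favouring the same or listed classes, passing on generation and kind.
; Pending generation is randomly cancelled with odds rising by generation, tapering growth.
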(event `self.ReceiveBeginPlay`
  (`self.CheckOverlap` (`self.DistanzaAutodistruzione`))
  (`KismetArrayLibrary.Array_Add` (`/Game/LOGIC/Main/BP_MainGameMode.LeafBuds` (cast `/Game/LOGIC/Main/BP_MainGameMode` (`GameplayStatics.GetGameMode`) :!pure true)) self))

(event `Set Reward Not Available`
  (set `self.Reward Available` false))

(event `SetGeneration`
  (params (Generation :type Integer))
  (bind _output_get (set `self.Generazione` Generation))
  (if (< (`KismetMathLibrary.RandomFloat`) (* (`self.ProbabilitàMorte`) (`KismetMathLibrary.FClamp` (/ (`KismetMathLibrary.Conv_IntToDouble` _output_get) 10.0))))
    (set `self.PendingGeneration` false)))

(event `SelectKind`
  (params (ParentKind :type Integer)))

(event `GenerateChildren`
  (bind _curbud (`self.CurBud`))
  (bind _angolocono (`self.AngoloCono`))
  (bind _figlimin (`self.FigliMin`))
  (bind _figlimax (`self.FigliMax`))
  (bind _returnvalue (`KismetMathLibrary.GreaterGreater_VectorRotator` (`KismetMathLibrary.VLerp` (`KismetMathLibrary.Vector_Normal2D` (`self.K2_GetActorLocation`)) (`self.GetActorForwardVector`) 0.5) (`KismetMathLibrary.MakeRotator` 0.0 0.0 (`KismetMathLibrary.RandomFloatInRange` (- 0.0 _angolocono) _angolocono))))
  (set `self.PendingGeneration` false)
  (for _ (range 1 (+ (`KismetMathLibrary.Clamp` (+ (`KismetMathLibrary.RandomIntegerInRange` _figlimin _figlimax) (`KismetMathLibrary.RandomIntegerInRange` _figlimin _figlimax)) (`self.FigliMin`) (`self.FigliMax`)) 1))
    (bind _returnvalue_2 (`|SpawnActorFromClass` (`self.GetRandomClass`) (`KismetMathLibrary.MakeTransform` (+ (`self.K2_GetActorLocation`) (* _returnvalue (`KismetMathLibrary.RandomFloatInRange` (`self.DistanzaMinima`) (`self.LunghezzaInternaCono`)))) (`KismetMathLibrary.Conv_VectorToRotator` _returnvalue)) "Undefined" "OverrideRootScale" null null))
    (bind _asbp_bud (cast `/Game/LOGIC/BP_Bud` _returnvalue_2))
    (set `self.CurBud` _asbp_bud)
    (`/Engine/EditorBlueprintResources/StandardMacros.IsValid` _curbud
      (:`Is Valid`
        (`self.SetGeneration` _curbud (+ (`self.Generazione`) 1))
        (`/Engine/EditorBlueprintResources/StandardMacros.IsValid` _curbud
          (:`Is Valid`
            (`self.SelectKind` _curbud (`self.Kind`))))))))

(fn `CheckOverlap`
  (params (Radius :type "Float (single-precision)"))
  (bind _returnvalue (`self.K2_GetActorLocation`))
  (bind (_outhit _returnvalue_2) (`KismetSystemLibrary.SphereTraceSingleForObjects` _returnvalue _returnvalue Radius (`|MakeArray` "ObjectTypeQuery2" :!type "EObjectTypeQuery Enum")))
  (if _returnvalue_2
    (if false
      (`PrimitiveComponent.SetMaterial` (`self.Sphere`) 0 "/Engine/VREditor/BasicMeshes/MI_Cube_03.MI_Cube_03")
      (else
        (`self.K2_DestroyActor`))))
  (return))

(fn `GetRandomClass`
  (returns (ReturnValue :type "Actor Class Reference"))
  (bind _classifigli (`self.ClassiFigli`))
  ;[1 1 1] Comment
  (return (select `bool` (<= (`KismetMathLibrary.RandomFloat`) (`self.ProbabilitàStessaClasse`)) :`false` (`|GetArrayItem` _classifigli (`KismetMathLibrary.RandomIntegerInRange` 0 (- (`KismetArrayLibrary.Array_Length` _classifigli) 1))) :`true` (`GameplayStatics.GetObjectClass` self) :!type "Actor Class Reference")))

(fn `UserConstructionScript`)