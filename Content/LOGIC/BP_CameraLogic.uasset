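; BP_CameraLogic drives a single camera actor in the level, found by class on BeginPlay.
; Every tick it smoothly turns that camera toward the player pawn with a partial rotation lerp along the shortest path.
; CE_MoveCamera slides the camera horizontally to a given location on a timeline, keeping its current height.
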(event `self.ReceiveBeginPlay`
  (bind _returnvalue (`GameplayStatics.GetActorOfClass` "/Script/Engine.CameraActor"))
  (set `self.Camera` _returnvalue))

(event `self.ReceiveTick`
  (params (DeltaSeconds :type "Float (single-precision)"))
  (bind _camera (`self.Camera`))
  (bind _output_get (set `self.LestRot` (`self.K2_GetActorRotation` _camera)))
  (`self.K2_SetActorRotation` _camera (`KismetMathLibrary.RLerp` _output_get (`KismetMathLibrary.Conv_VectorToRotator` (- (`self.K2_GetActorLocation` (`GameplayStatics.GetPlayerPawn` 0)) (`self.K2_GetActorLocation` _camera))) 0.1 true) false))

(event `CE_MoveCamera`
  (params (TargetLocation :type "Vector Structure"))
  (bind _camera (`self.Camera`))
  (bind (_returnvalue_x _returnvalue_y _returnvalue_z) (`KismetMathLibrary.BreakVector` (`self.K2_GetActorLocation` _camera)))
  (set `self.TargetLocation` (`KismetMathLibrary.MakeVector` (.x TargetLocation) (.y TargetLocation) _returnvalue_z))
  (set `self.StartLocation` (`self.K2_GetActorLocation` _camera))
  (bind (_direction _linear) (`Timeline|CameraSlide` :!via `PlayFromStart`)
    (:`Update`
      (`self.K2_SetActorLocation` (`self.Camera`) (`KismetMathLibrary.VLerp` (`self.StartLocation`) (`self.TargetLocation`) _linear) false false))))

(fn `UserConstructionScript`)