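; BP_PlayerCharacter is the player character, providing axis-driven movement and look, plus an E key that calls GenerateOnce on BP_MainGameMode.
; BeginPlay caches the BP_CameraLogic actor, and Tick draws a debug line trace between Actor0 and Actor1 when both are valid.
; An unwired raycast chain would pick ConnectionNode-tagged actors via FlipFlop and pass pairs to the game mode's CreateConnection, but it never runs.
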(event `self.ReceiveBeginPlay`
  (bind _returnvalue (`GameplayStatics.GetActorOfClass` "/Game/LOGIC/BP_CameraLogic.BP_CameraLogic_C"))
  (set `self.BPCamera` _returnvalue))

(event `InputAxis|MoveUpDown`
  (params (AxisValue :type "Float (single-precision)"))
  (`self.AddMovementInput` (`self.GetActorForwardVector`) AxisValue))

(event `InputAxis|LookUpDown`
  (params (AxisValue :type "Float (single-precision)"))
  (`self.AddControllerPitchInput` AxisValue))

(event `self.ReceiveTick`
  (params (DeltaSeconds :type "Float (single-precision)"))
  (if (and (`KismetSystemLibrary.IsValid` (`self.Actor0`)) (`KismetSystemLibrary.IsValid` (`self.Actor1`)))
    (`KismetSystemLibrary.LineTraceSingle` :`Start` (`self.K2_GetActorLocation` (`self.Actor0`)) :`End` (`self.K2_GetActorLocation` (`self.Actor1`)) :`TraceChannel` "TraceTypeQuery1" :`DrawDebugType` "ForOneFrame")))

(event `InputAxis|MoveRightLeft`
  (params (AxisValue :type "Float (single-precision)"))
  (`self.AddMovementInput` (`self.GetActorRightVector`) AxisValue))

(event `InputAxis|LookRightLeft`
  (params (AxisValue :type "Float (single-precision)"))
  (`self.AddControllerYawInput` AxisValue))

(event `Key|E`
  (params (Key :type "Key Structure"))
  (:`Pressed`
    (`/Game/LOGIC/Main/BP_MainGameMode.GenerateOnce` (cast `/Game/LOGIC/Main/BP_MainGameMode` (`GameplayStatics.GetGameMode`) :!pure true))))

(event `InputAction|Connect`
  (params (Key :type "Key Structure")))

(fn `UserConstructionScript`)